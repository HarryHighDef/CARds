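; RoadBP is a procedural road segment that spawns the next random piece at its socket, extending the track when a vehicle hits its trigger cube.
; Each piece carries estimated speed and remaining count forward, with speed affecting piece choice.
; A swept box rejects overlapping candidates, and exhausted options backtrack to the previous piece.
; Accumulated twist switches selection to the most upright exit, or eventually a yaw-only spawn.
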(event OnComponentBeginOverlap(Cube)
  (params (OverlappedComponent :type Primitive%20Component%20Object%20Reference) (OtherActor :type Actor%20Object%20Reference) (OtherComp :type Primitive%20Component%20Object%20Reference) (OtherBodyIndex :type Integer) (bFromSweep :type Boolean) (SweepResult :type Hit%20Result%20Structure%20%28by%20ref%29))
  (Utilities|Casting|CastToVehicleBlueprint OtherActor)
  (if (Variables|Default|GetReady)
    (bind _output_get (Variables|Default|SetRemaining%20Segments 50))
    (CallFunction|AddNextPiece _output_get)
    (else
      (Components|DestroyComponent (Variables|Default|GetCube)))))

(event Custom|DelayedNextPiece
  (CallFunction|AddNextPiece (Variables|Default|GetRemaining%20Segments)))

(event Custom|AddOne
  (CallFunction|AddNextPiece 1))

(event EventBeginPlay
  (CallFunction|CalculateSpeed)
  (if (> (Variables|Default|GetRemaining%20Segments) 0)
    (Utilities|Time|SetTimerbyEvent (delegate Custom|DelayedNextPiece) 0.01)
    (else
      (Utilities|Time|SetTimerbyEvent (EventDispatchers|CreateEvent :!event MoveCubeBack) 0.1)))
  (Utilities|Time|SetTimerbyEvent (EventDispatchers|CreateEvent :!event K2DestroyActor) 8e+01))

(fn ConstructionScript
  (bind (_origin _boxextent) (Collision|GetActorBounds true false))
  (Transformation|SetRelativeTransform (Variables|Default|GetNextConnector) (Variables|Default|GetNextSocket) false false)
  (bind _returnvalue (AddComponent|AddBoxComponent false))
  (Transformation|SetWorldLocationAndRotation _returnvalue _origin "0, 0, 0" false false)
  (Components|Box|SetBoxExtent _returnvalue _boxextent true))

(fn CalculateSpeed
  (bind _prevspeeed (Variables|Default|GetPrevSpeeed))
  (bind _estimatedaccel (Variables|Default|GetEstimatedAccel))
  (bind _returnvalue (+ _prevspeeed _estimatedaccel))
  (CallFunction|CalculateTwist)
  (if (>= _returnvalue 4e+01)
    (Variables|Default|SetEstimatedSpeed (Math|Float|MapRangeClamped _returnvalue 4e+01 8e+01 4e+01 6e+01))
    (else
      (Variables|Default|SetEstimatedSpeed _returnvalue))))

(fn AddNextPiece
  (params (RemainingSegments :type Integer))
  (bind _road_types (Variables|Default|GetRoad%20Types))
  (bind _returnvalue (Utilities|Array|Length _road_types))
  (if (> (Variables|Default|GetUntwist) 0)
    (CallFunction|CalculateUntwist)
    (elif (> (Utilities|Array|Length (Variables|Default|GetRoad%20Types)) 0)
      (bind _returnvalue_2 (Game|SpawnActorfromClass (Utilities|Array|Get(acopy) _road_types (Math|Random|RandomInteger (Math|Integer|Min(Integer) _returnvalue (Math|Integer|SelectInt _returnvalue 12 (< (Variables|Default|GetEstimatedSpeed) 4e+01))))) (Math|Transform|ComposeTransforms (Variables|Default|GetNextSocket) (Transformation|GetWorldTransform (Variables|Default|GetDefaultSceneRoot))) "Undefined" 0 (Variables|Default|GetEstimatedSpeed) (- RemainingSegments 1) 0 self 0))
      (Utilities|Array|RemoveItem (Variables|Default|GetRoad%20Types) (Utilities|GetClass _returnvalue_2))
      (bind _foundoverlaps (CallFunction|CheckforClipping _returnvalue_2))
      (if _foundoverlaps
        (Actor|DestroyActor _returnvalue_2)
        (CallFunction|AddNextPiece (Variables|Default|GetRemaining%20Segments))
        (else
          (bind _cube (Variables|Default|GetCube)
            (:then
              (Components|DestroyComponent _cube))
            (:else
              _))
          (Variables|Default|SetReady true)))
      (else
        (Collision|SetActorEnableCollision false)
        (CallFunction|DelayedNextPiece (Variables|Default|GetPrevious))
        (Actor|DestroyActor)))))

(fn CalculateUntwist
  (bind _possiblepaths (LocalVariables|GetPossiblePaths))
  (bind _possiblepaths_2 (LocalVariables|GetPossiblePaths))
  (bind _nextsocket (Variables|Default|GetNextSocket))
  (bind _defaultsceneroot (Variables|Default|GetDefaultSceneRoot))
  (bind _returnvalue (Transformation|GetWorldTransform _defaultsceneroot))
  (bind _returnvalue_2 (Math|Transform|ComposeTransforms _nextsocket _returnvalue))
  (if (> (Variables|Default|GetUntwist) 10)
    (Game|SpawnActorfromClass "RoadBP_C" (Math|Transform|MakeTransform (.location _returnvalue_2) (Math|Rotator|MakeRotator 0.0 0.0 (.yaw (.rotation _returnvalue_2))) "1,1,1") "Undefined" 0 (Variables|Default|GetEstimatedSpeed) (- (Variables|Default|GetRemaining%20Segments) 1) 0 self 0)
    (Components|DestroyComponent (Variables|Default|GetCube))
    (Variables|Default|SetReady true)
    (else
      (for _array_element (Variables|Default|GetRoad%20TypesUntwist)
        (bind _returnvalue_3 (Game|SpawnActorfromClass _array_element (Math|Transform|ComposeTransforms (Variables|Default|GetNextSocket) (Transformation|GetWorldTransform (Variables|Default|GetDefaultSceneRoot))) "Undefined" 0 (Variables|Default|GetEstimatedSpeed) (Math|Integer|Min(Integer) (Variables|Default|GetRemaining%20Segments) 1) (Variables|Default|GetUntwist) self 0))
        (bind _foundoverlaps (CallFunction|CheckforClipping _returnvalue_3))
        (if _foundoverlaps
          (Actor|DestroyActor _returnvalue_3)
          (else
            (Utilities|Array|Add (LocalVariables|GetPossiblePaths) _returnvalue_3)
            (Transformation|SetActorLocation _returnvalue_3 "0, 0, 0" false false))))
      (if (> (Utilities|Array|Length _possiblepaths) 0)
        (Utilities|Array|Shuffle _possiblepaths)
        (for (_array_element_2 _array_index) _possiblepaths_2
          (if (> (CallFunction|GetTwistEnd _array_element_2) (CallFunction|GetTwistEnd (Utilities|Array|Get(acopy) _possiblepaths_2 (LocalVariables|GetBestUntwist))))
            (LocalVariables|SetBestUntwist _array_index)))
        (Utilities|Array|RemoveItem (Variables|Default|GetRoad%20TypesUntwist) (Utilities|GetClass (Utilities|Array|Get(acopy) _possiblepaths_2 (LocalVariables|GetBestUntwist))))
        (Variables|RoadBP_C|SetRemaining%20Segments (Utilities|Array|Get(acopy) _possiblepaths_2 (LocalVariables|GetBestUntwist)) (- (Variables|Default|GetRemaining%20Segments) 1))
        (Transformation|SetActorLocation (Utilities|Array|Get(acopy) _possiblepaths_2 (LocalVariables|GetBestUntwist)) (.location (Math|Transform|ComposeTransforms (Variables|Default|GetNextSocket) (Transformation|GetWorldTransform (Variables|Default|GetDefaultSceneRoot)))) false false)
        (Utilities|Array|RemoveIndex _possiblepaths_2 (LocalVariables|GetBestUntwist))
        (Components|DestroyComponent (Variables|Default|GetCube))
        (Variables|Default|SetReady true)
        (for _array_element_3 (LocalVariables|GetPossiblePaths)
          (Actor|DestroyActor _array_element_3))
        (else
          (Collision|SetActorEnableCollision false)
          (CallFunction|DelayedNextPiece (Variables|Default|GetPrevious))
          (Actor|DestroyActor))))))

(fn GetTwist
  (return (Class|KismetMathLibrary|DegAcos (Math|Vector|DotProduct (Math|Vector|GetUpVector (Transformation|GetActorRotation)) "0, 0,1.000000"))))

(fn GetTwistEnd
  (Development|PrintString (Utilities|String|Append (Utilities|GetDisplayName self) " End Twist of: " (Utilities|String|ToString(Float) 0.0)))
  (return (Math|Vector|DotProduct (Math|Vector|GetUpVector (.rotation (Math|Transform|ComposeTransforms (Variables|Default|GetNextSocket) (Transformation|GetWorldTransform (Variables|Default|GetDefaultSceneRoot))))) "0, 0,1.000000")))

(fn CalculateTwist
  (bind _returnvalue (CallFunction|GetTwist))
  (bind _returnvalue_2 (Transformation|GetActorRotation))
  (bind _estimatedspeed (Variables|Default|GetEstimatedSpeed))
  (bind _returnvalue_3 (Math|Float|Max(Float) _estimatedspeed 1.0))
  (bind _returnvalue_4 (/ _returnvalue_3 1e+02))
  (Variables|Default|SetUntwist (* (+ (Variables|Default|GetUntwist) (Math|Conversions|ToInteger(Boolean) (or (and (> (Variables|Default|GetUntwist) 0) (> _returnvalue 3.0)) (> _returnvalue 3e+01)))) (Math|Conversions|ToInteger(Boolean) (or (and (> (Variables|Default|GetUntwist) 0) (> _returnvalue 3.0)) (> _returnvalue 3e+01)))))
  (if (< (CallFunction|GetTwist) 5.0)
    (Transformation|SetActorRotation (Math|Rotator|MakeRotator (Math|Interpolation|FInterpTo (.roll _returnvalue_2) 0.0 _returnvalue_4 1.0) (Math|Interpolation|FInterpTo (.pitch _returnvalue_2) 0.0 _returnvalue_4 1.0) (.yaw _returnvalue_2)))))

(fn CheckforClipping
  (bind _cube (Variables|Default|GetCube))
  (bind _cube_2 (Variables|Default|GetCube))
  (bind _cube_3 (Variables|Default|GetCube))
  (Transformation|AttachComponentToComponent _cube (Variables|Default|GetDefaultSceneRoot) "None" "SnapToTarget" "SnapToTarget" "KeepRelative" true)
  (Transformation|SetRelativeLocation _cube "0,250.000000, 0" false false)
  (for _index (range 0 10)
    (Transformation|SetWorldTransform _cube_2 (Math|Transform|Lerp(Transform) (Math|Transform|ComposeTransforms (Math|Transform|MakeTransform "0,250.000000, 0" "0, 0, 0" "1,5.000000,1") (Transformation|GetWorldTransform (Variables|Default|GetDefaultSceneRoot))) (Math|Transform|ComposeTransforms (Math|Transform|MakeTransform "0,250.000000, 0" "0, 0, 0" "1,5.000000,1") (Variables|Default|GetNextSocket)) (* _index 0.1)) false false)
    (bind _output_get (LocalVariables|SetClips (Collision|GetOverlappingActors _cube_2 "RoadBP_C" :!class /Script/Engine.PrimitiveComponent)))
    (Utilities|Array|RemoveItem _output_get (Variables|Default|GetPrevious))
    (if (> (Utilities|Array|Length _output_get) 1)
      (return true)))
  (Transformation|AttachComponentToComponent _cube_3 (Variables|Default|GetNextConnector) "None" "SnapToTarget" "SnapToTarget" "KeepRelative" true)
  (Transformation|SetRelativeLocation _cube_3 "0,250.000000, 0" false false)
  (return false))

(fn MoveCubeBack
  (bind _cube (Variables|Default|GetCube))
  (Variables|Default|SetReady true)
  (Variables|Default|SetCubeTarget (Variables|Default|GetPrevious))
  (for _index (range 0 9)
    (Variables|Default|SetCubeTarget (Variables|RoadBP_C|GetPrevious (Variables|Default|GetCubeTarget))))
  (Transformation|SetWorldTransform _cube (Math|Transform|ComposeTransforms (Math|Transform|MakeTransform "0,250.000000, 0" "0, 0, 0" "1,5.000000,1") (Transformation|GetWorldTransform (Variables|RoadBP_C|GetNextConnector (Variables|Default|GetCubeTarget)))) false false)
  (Collision|SetCollisionResponsetoAllChannels _cube "ECR_Overlap"))