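; Hover vehicle Blueprint that floats on four downward thrusters, recalculating their strength every tick.
; Each thruster line-traces along its forward vector and pushes harder the closer the hit, plus damping from its movement along that axis since last frame.
; A second pass adds shared thrust from the averaged hit distance, which carries over between frames, and stores positions for the next tick.
; Debug trace drawing and a print remain active.
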(event EventBeginPlay
  (Variables|Default|SetDownThrusters (Utilities|Array|MakeArray (Variables|Default|GetDownThruster1) (Variables|Default|GetDownThruster2) (Variables|Default|GetDownThruster3) (Variables|Default|GetDownThruster4))))

(event Collision|EventActorBeginOverlap
  (params (OtherActor :type Actor%20Object%20Reference)))

(event EventTick
  (params (DeltaSeconds :type Float%20%28single-precision%29))
  (Variables|Default|SetDelta DeltaSeconds)
  (CallFunction|ThurstHandle))

(fn ConstructionScript)

(fn ThurstHandle
  (for (_array_element _array_index) (Variables|Default|GetDownThrusters)
    (bind (_outhit _returnvalue) (Collision|LineTraceByChannel (Transformation|GetWorldLocation _array_element) (+ (Transformation|GetWorldLocation _array_element) (* (Math|Vector|GetForwardVector _array_element) 5e+02)) "TraceTypeQuery1" false (Utilities|Array|MakeArray 0) "ForDuration"))
    (if _returnvalue
      (LocalVariables|SetAverageDist (+ (LocalVariables|GetAverageDist) (.Distance (Collision|BreakHitResult _outhit))))
      (Variables|/Script/Engine.PhysicsThrusterComponent|SetThrustStrength _array_element (Math|Float|Clamp(Float) (/ 8.75e+03 (/ (.Distance (Collision|BreakHitResult _outhit)) 1e+02)) 1e+02 2e+04))
      (Development|PrintString "Hello")
      (Variables|/Script/Engine.PhysicsThrusterComponent|SetThrustStrength _array_element (+ (Variables|/Script/Engine.PhysicsThrusterComponent|GetThrustStrength _array_element) (Math|Float|MapRangeClamped (/ (* (Math|Vector|VectorLengthSquared (- (Transformation|GetWorldLocation _array_element) (Utilities|Array|Get(acopy) (Variables|Default|GetDownPositions) _array_index))) (Math|Float|Max(Float) (Math|Vector|DotProduct (Math|Vector|Normalize (- (Transformation|GetWorldLocation _array_element) (Utilities|Array|Get(acopy) (Variables|Default|GetDownPositions) _array_index))) (Math|Vector|GetForwardVector _array_element)) 0.0)) (Variables|Default|GetDelta)) 0.0 1e+05 0.0 2e+03)))
      (else
        (Variables|/Script/Engine.PhysicsThrusterComponent|SetThrustStrength _array_element 1e+03))))
  (Utilities|Array|Clear (Variables|Default|GetDownPositions))
  (bind _output_get (LocalVariables|SetAverageDist (/ (LocalVariables|GetAverageDist) 4.0)))
  (for _array_element_2 (Variables|Default|GetDownThrusters)
    (if (> _output_get 0.0)
      (Variables|/Script/Engine.PhysicsThrusterComponent|SetThrustStrength _array_element_2 (+ (Variables|/Script/Engine.PhysicsThrusterComponent|GetThrustStrength _array_element_2) (Math|Float|Clamp(Float) (/ 8.75e+03 (/ _output_get 1e+02)) 1e+02 2e+04)))
      (else
        (Variables|/Script/Engine.PhysicsThrusterComponent|SetThrustStrength _array_element_2 1e+03)))
    (Utilities|Array|Add (Variables|Default|GetDownPositions) (Transformation|GetWorldLocation _array_element_2))))